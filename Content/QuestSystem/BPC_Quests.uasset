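; Quest component that tracks the active quest's kill and collect objectives and shows them on a WB_QuestHud widget created at BeginPlay.
; EliminateEnemy removes actors from a working list until empty, while CollectItem matches the chest to open; both write completion back by reference and notify the HUD.
; Only elimination calls ObjectiveCompleted, which clears the quest when its count reaches the objective total.
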(event Custom|SetTextQuest's
  (Rendering|Components|TextRender|SetText (Variables|/Game/QuestSystem/WB_QuestHud.WB_QuestHud_C|GetActiveQuestText (Variables|Default|GetQuestHud)) (Utilities|Text|ToText(String) (.name (Variables|Default|GetactiveQuest)))))

(event Custom|SetObjectives
  (Default|FillObjectives (Variables|Default|GetQuestHud) (.objectives (Variables|Default|GetactiveQuest))))

(event Custom|Eliminate%20Enemy
  (params (actor :type Actor%20Object%20Reference))
  (for _array_element (.objectives (Variables|Default|GetactiveQuest))
    (if (and (not (.Completed (Utilities|Struct|BreakS_QuestObjective _array_element))) (.isEliminateEnemyObjective (Utilities|Struct|BreakS_QuestObjective _array_element)))
      (if (!= (Utilities|Array|Length (Variables|Default|GetActors%20to%20Eliminate)) 0)
        _
        (else
          (bind _output_get (Variables|Default|SetActors%20to%20Eliminate (.ActorsToEliminate (Utilities|Struct|BreakS_QuestObjective _array_element))))))
      (Utilities|Array|RemoveItem _output_get actor)
      (|SetBy-RefVar _array_element (Utilities|Struct|MakeS_QuestObjective (.NameAim (Utilities|Struct|BreakS_QuestObjective _array_element)) false (Variables|Default|GetActors%20to%20Eliminate) (.CollectToOpen (Utilities|Struct|BreakS_QuestObjective _array_element)) (.isEliminateEnemyObjective (Utilities|Struct|BreakS_QuestObjective _array_element)) (.isCollectItemObjective (Utilities|Struct|BreakS_QuestObjective _array_element))))
      (if (== (Utilities|Array|Length (Variables|Default|GetActors%20to%20Eliminate)) 0)
        (|SetBy-RefVar _array_element (Utilities|Struct|MakeS_QuestObjective (.NameAim (Utilities|Struct|BreakS_QuestObjective _array_element)) true (Variables|Default|GetActors%20to%20Eliminate) (.CollectToOpen (Utilities|Struct|BreakS_QuestObjective _array_element)) (.isEliminateEnemyObjective (Utilities|Struct|BreakS_QuestObjective _array_element)) (.isCollectItemObjective (Utilities|Struct|BreakS_QuestObjective _array_element))))
        (Default|CompleteObjectives (Variables|Default|GetQuestHud) _array_element)
        (CallFunction|ObjectiveCompleted)))))

(event Custom|CollectItem
  (params (Chest :type Actor%20Object%20Reference))
  (for _array_element (.objectives (Variables|Default|GetactiveQuest))
    (if (and (.isCollectItemObjective (Utilities|Struct|BreakS_QuestObjective _array_element)) (== Chest (.CollectToOpen (Utilities|Struct|BreakS_QuestObjective _array_element))))
      (|SetBy-RefVar _array_element (Utilities|Struct|MakeS_QuestObjective (.NameAim (Utilities|Struct|BreakS_QuestObjective _array_element)) true (.ActorsToEliminate (Utilities|Struct|BreakS_QuestObjective _array_element)) 0 (.isEliminateEnemyObjective (Utilities|Struct|BreakS_QuestObjective _array_element)) (.isCollectItemObjective (Utilities|Struct|BreakS_QuestObjective _array_element))))
      (Default|CompleteObjectives (Variables|Default|GetQuestHud)))))

(event Custom|Objective%20Completed
  (Math|Integer|IncrementInt (Variables|Default|GetobjectiveCompletedInt)
    (:%20%20
      (if (>= (Variables|Default|GetobjectiveCompletedInt) (Utilities|Array|Length (.objectives (Variables|Default|GetactiveQuest))))
        (Variables|Default|SetactiveQuest "")
        (Variables|Default|SetobjectiveCompletedInt 0)))))

(event EventBeginPlay
  (bind _returnvalue (UserInterface|CreateWidget "/Game/QuestSystem/WB_QuestHud.WB_QuestHud_C"))
  (bind _output_get (Variables|Default|SetQuestHud _returnvalue))
  (UserInterface|Viewport|AddtoViewport _output_get 0))