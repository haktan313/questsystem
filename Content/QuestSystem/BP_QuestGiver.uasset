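; Quest giver actor that lets the third-person character view the quests it offers through a quest HUD.
; A sphere overlap shows or hides its widget component as the character enters or leaves.
; TakeQuest toggles a WB_QuestGiver screen, filling it from the Quests array and passing itself as a back-reference.
; Opening enables the cursor with Game and UI input, while toggling again or calling Close removes the screen and restores game-only input.
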(event OnComponentBeginOverlap(Sphere)
  (params (OverlappedComponent :type Primitive%20Component%20Object%20Reference) (OtherActor :type Actor%20Object%20Reference) (OtherComp :type Primitive%20Component%20Object%20Reference) (OtherBodyIndex :type Integer) (bFromSweep :type Boolean) (SweepResult :type Hit%20Result%20Structure%20%28by%20ref%29))
  (bind _asbp_third_person_character (Utilities|Casting|CastToBP_ThirdPersonCharacter OtherActor))
  (Variables|Default|SetAs%20BP%20Third%20Person%20Character _asbp_third_person_character)
  (Rendering|SetVisibility (Variables|Default|GetWidget) true false))

(event OnComponentEndOverlap(Sphere)
  (params (OverlappedComponent :type Primitive%20Component%20Object%20Reference) (OtherActor :type Actor%20Object%20Reference) (OtherComp :type Primitive%20Component%20Object%20Reference) (OtherBodyIndex :type Integer))
  (Utilities|Casting|CastToBP_ThirdPersonCharacter OtherActor)
  (Rendering|SetVisibility (Variables|Default|GetWidget) false false))

(event Custom|Close
  (bind _returnvalue (Game|GetPlayerController 0))
  (Variables|Default|SetisQuestHUDOpen? false)
  (Widget|RemovefromParent (Variables|Default|GetquestHUD))
  (Variables|/Script/Engine.PlayerController|SetbShowMouseCursor _returnvalue false)
  (Input|SetInputModeGameOnly _returnvalue false))

(event EventBeginPlay)

(event Collision|EventActorBeginOverlap
  (params (OtherActor :type Actor%20Object%20Reference)))

(event EventTick
  (params (DeltaSeconds :type Float%20%28single-precision%29)))

(event EventTakeQuest
  (bind _returnvalue (Game|GetPlayerController 0))
  (bind _returnvalue_2 (Game|GetPlayerController 0))
  (if (not (Variables|Default|GetisQuestHUDOpen?))
    (bind _returnvalue_3 (UserInterface|CreateWidget "/Game/QuestSystem/WB_QuestGiver.WB_QuestGiver_C"))
    (bind _output_get (Variables|Default|SetquestHUD _returnvalue_3))
    (UserInterface|Viewport|AddtoViewport _output_get 0)
    (Variables|Default|SetisQuestHUDOpen? true)
    (Variables|/Script/Engine.PlayerController|SetbShowMouseCursor _returnvalue_2 true)
    (Input|SetInputModeGameandUI _returnvalue_2 0 "DoNotLock" true false)
    (Variables|/Game/QuestSystem/WB_QuestGiver.WB_QuestGiver_C|SetquestGiveBP (Variables|Default|GetquestHUD) self)
    (for _array_element (Variables|Default|Getquests)
      (Default|AddQuest (Variables|Default|GetquestHUD) _array_element))
    (else
      (Variables|Default|SetisQuestHUDOpen? false)
      (Widget|RemovefromParent (Variables|Default|GetquestHUD))
      (Variables|/Script/Engine.PlayerController|SetbShowMouseCursor _returnvalue false)
      (Input|SetInputModeGameOnly _returnvalue false))))

(fn ConstructionScript)